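; Player stats component that tracks current and max health and stamina for BP_ThirdPersonCharacter.
; It caches the owning character a tick after BeginPlay, and each change function pushes the new ratio to its HUD bar.
; Regen clamps to max; decreases return whether health is depleted, even DecreaseStamina, which checks CurrentHealth.
; IncreaseMaxStamina raises MaxHealth instead of MaxStamina.
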(event EventBeginPlay
  (Utilities|FlowControl|DelayUntilNextTick)
  (bind _asbp_third_person_character (Utilities|Casting|CastToBP_ThirdPersonCharacter (Components|GetOwner)))
  (Variables|Default|SetPlayer%20Character%20BP _asbp_third_person_character)
  (Progress|SetPercent (Variables|/Game/UI/WB_HUD.WB_HUD_C|GetStaminaBar (Variables|/Game/ThirdPerson/Blueprints/BP_ThirdPersonCharacter.BP_ThirdPersonCharacter_C|GetHud%20Widget (Variables|Default|GetPlayer%20Character%20BP))) (/ (Variables|Stamina|GetCurrent%20Stamina) (Variables|Stamina|GetMax%20Stamina)))
  (Progress|SetPercent (Variables|/Game/UI/WB_HUD.WB_HUD_C|GetHealthBar (Variables|/Game/ThirdPerson/Blueprints/BP_ThirdPersonCharacter.BP_ThirdPersonCharacter_C|GetHud%20Widget (Variables|Default|GetPlayer%20Character%20BP))) (/ (Variables|Health|GetCurrent%20Health) (Variables|Health|GetMax%20Health))))

(fn DecreaseHealth
  (params (Damage :type Float%20%28double-precision%29))
  (bind _output_get (Variables|Health|SetCurrent%20Health (- (Variables|Health|GetCurrent%20Health) Damage)))
  (Progress|SetPercent (Variables|/Game/UI/WB_HUD.WB_HUD_C|GetHealthBar (Variables|/Game/ThirdPerson/Blueprints/BP_ThirdPersonCharacter.BP_ThirdPersonCharacter_C|GetHud%20Widget (Variables|Default|GetPlayer%20Character%20BP))) (/ _output_get (Variables|Health|GetMax%20Health)))
  (if (<= (Variables|Health|GetCurrent%20Health) 0.0)
    (return true)
    (else
      (return false))))

(fn IncreaseMaxHealth
  (params (Health%20Increase :type Float%20%28double-precision%29))
  (Variables|Health|SetMax%20Health (+ (Variables|Health|GetMax%20Health) Health%20Increase))
  (Progress|SetPercent (Variables|/Game/UI/WB_HUD.WB_HUD_C|GetHealthBar (Variables|/Game/ThirdPerson/Blueprints/BP_ThirdPersonCharacter.BP_ThirdPersonCharacter_C|GetHud%20Widget (Variables|Default|GetPlayer%20Character%20BP))) (/ (Variables|Health|GetCurrent%20Health) (Variables|Health|GetMax%20Health))))

(fn DecreaseStamina
  (params (Depletion :type Float%20%28double-precision%29))
  (Variables|Stamina|SetCurrent%20Stamina (- (Variables|Stamina|GetCurrent%20Stamina) Depletion))
  (Progress|SetPercent (Variables|/Game/UI/WB_HUD.WB_HUD_C|GetStaminaBar (Variables|/Game/ThirdPerson/Blueprints/BP_ThirdPersonCharacter.BP_ThirdPersonCharacter_C|GetHud%20Widget (Variables|Default|GetPlayer%20Character%20BP))) (/ (Variables|Stamina|GetCurrent%20Stamina) (Variables|Stamina|GetMax%20Stamina)))
  (if (<= (Variables|Health|GetCurrent%20Health) 0.0)
    (return true)
    (else
      (return false))))

(fn IncreaseMaxStamina
  (params (Stamina%20Increase :type Float%20%28double-precision%29))
  (Variables|Health|SetMax%20Health (+ (Variables|Health|GetMax%20Health) Stamina%20Increase))
  (Progress|SetPercent (Variables|/Game/UI/WB_HUD.WB_HUD_C|GetStaminaBar (Variables|/Game/ThirdPerson/Blueprints/BP_ThirdPersonCharacter.BP_ThirdPersonCharacter_C|GetHud%20Widget (Variables|Default|GetPlayer%20Character%20BP))) (/ (Variables|Stamina|GetCurrent%20Stamina) (Variables|Stamina|GetMax%20Stamina))))

(fn IncreaseHealth
  (params (Health%20Regen :type Float%20%28double-precision%29))
  (Variables|Health|SetCurrent%20Health (+ (Variables|Health|GetCurrent%20Health) Health%20Regen))
  (if (> (Variables|Health|GetCurrent%20Health) (Variables|Health|GetMax%20Health))
    (Variables|Health|SetCurrent%20Health (Variables|Health|GetMax%20Health)))
  (Progress|SetPercent (Variables|/Game/UI/WB_HUD.WB_HUD_C|GetHealthBar (Variables|/Game/ThirdPerson/Blueprints/BP_ThirdPersonCharacter.BP_ThirdPersonCharacter_C|GetHud%20Widget (Variables|Default|GetPlayer%20Character%20BP))) (/ (Variables|Health|GetCurrent%20Health) (Variables|Health|GetMax%20Health))))

(fn IncreaseStamina
  (params (Stamina%20Regen :type Float%20%28double-precision%29))
  (Variables|Stamina|SetCurrent%20Stamina (+ (Variables|Stamina|GetCurrent%20Stamina) Stamina%20Regen))
  (if (> (Variables|Stamina|GetCurrent%20Stamina) (Variables|Stamina|GetMax%20Stamina))
    (Variables|Stamina|SetCurrent%20Stamina (Variables|Stamina|GetMax%20Stamina)))
  (Progress|SetPercent (Variables|/Game/UI/WB_HUD.WB_HUD_C|GetStaminaBar (Variables|/Game/ThirdPerson/Blueprints/BP_ThirdPersonCharacter.BP_ThirdPersonCharacter_C|GetHud%20Widget (Variables|Default|GetPlayer%20Character%20BP))) (/ (Variables|Stamina|GetCurrent%20Stamina) (Variables|Stamina|GetMax%20Stamina))))